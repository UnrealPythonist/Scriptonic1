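; First-person character Blueprint, named FPSController, handling movement, mouse look, a double jump and a dash.
; Movement axes follow control yaw only, while mouse axes feed controller yaw and pitch.
; A counter, reset on landing, caps jumps at two; it increments before its zero check, so presses launch upward instead of reaching Jump.
; Dash adds a large horizontal launch along the facing yaw, with no cooldown.
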(event EventOnLanded
  (params (Hit :type Hit%20Result%20Structure%20%28by%20ref%29))
  (Variables|Default|SetJump%20Count 0))

(event Input|ActionEvents|InputActionJump/DoubleJump
  (params (Key :type Key%20Structure))
  (bind _jump_count (Variables|Default|GetJump%20Count))
  (:Pressed
    (if (< _jump_count 2)
      (Math|Integer|IncrementInt _jump_count
        (:%20%20
          (if (== _jump_count 0)
            (Character|Jump)
            (else
              (Character|LaunchCharacter (+ (Transformation|GetVelocity) "0, 0,500.000000") false true)))))))
  (:Released
    (Character|StopJumping)))

(event Input|ActionEvents|InputActionDash
  (params (Key :type Key%20Structure))
  (:Pressed
    (Character|LaunchCharacter (* (Math|Vector|GetForwardVector (Math|Rotator|MakeRotator 0.0 0.0 (.yaw (Pawn|GetControlRotation :!class /Script/Engine.Pawn)))) 10000) false false)))

(event Input|AxisEvents|InputAxisHorizontal
  (params (AxisValue :type Float%20%28single-precision%29))
  (Pawn|Input|AddMovementInput (Math|Vector|GetRightVector (Math|Rotator|MakeRotator 0.0 0.0 (.yaw (Pawn|GetControlRotation :!class /Script/Engine.Pawn)))) AxisValue false))

(event Input|AxisEvents|InputAxisVertical
  (params (AxisValue :type Float%20%28single-precision%29))
  (Pawn|Input|AddMovementInput (Math|Vector|GetForwardVector (Math|Rotator|MakeRotator 0.0 0.0 (.yaw (Pawn|GetControlRotation :!class /Script/Engine.Pawn)))) AxisValue false))

(event Input|AxisEvents|InputAxisMouseLookHorizontal
  (params (AxisValue :type Float%20%28single-precision%29))
  (Pawn|Input|AddControllerYawInput AxisValue))

(event Input|AxisEvents|InputAxisMouseLookVertical
  (params (AxisValue :type Float%20%28single-precision%29))
  (Pawn|Input|AddControllerPitchInput AxisValue))

(fn ConstructionScript)